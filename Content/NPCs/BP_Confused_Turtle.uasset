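; BP_Confused_Turtle is an NPC turtle that keeps flipping between walking forwards and walking backwards until it overlaps a finish line.
; On BeginPlay, two looping timers with equal periods but staggered start delays both call SwitchAnimation, producing an uneven switching rhythm.
; SwitchAnimation checks the TurtleBody mesh's current anim instance and swaps its Animation Blueprint class between the two walks.
; Overlapping a BP_FinishLine pauses both timers, freezing whichever animation is active.
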(event EventBeginPlay
  (bind _self self)
  (bind _returnvalue (Utilities|Time|SetTimerbyFunctionName _self "SwitchAnimation" 1.5 true 1.0))
  (bind _returnvalue_2 (Utilities|Time|SetTimerbyFunctionName _self "SwitchAnimation" 1.5 true 1.5)))

(event Collision|EventActorBeginOverlap
  (params (OtherActor :type Actor%20Object%20Reference))
  (Utilities|Casting|CastToBP_FinishLine OtherActor)
  (Utilities|Time|PauseTimerbyHandle (stale EventBeginPlay _returnvalue))
  (Utilities|Time|PauseTimerbyHandle (stale EventBeginPlay _returnvalue_2)))

(event EventTick
  (params (DeltaSeconds :type Float%20%28single-precision%29)))

(fn ConstructionScript)

(fn SwitchAnimation
  (bind _turtlebody (Variables|Default|GetTurtleBody)
    (:then
      (bind _output_get (LocalVariables|SetCurrentAnimation (Components|SkeletalMesh|GetAnimInstance _turtlebody)))
      (Utilities|Casting|CastToBP_TurtleWalking _output_get
        (:then
          (Class|SkeletalMeshComponent|SetAnimClass _turtlebody "/Game/NPCs/BP_TurtleWalkingBackwards.BP_TurtleWalkingBackwards_C"))
        (:CastFailed
          (Class|SkeletalMeshComponent|SetAnimClass _turtlebody "/Game/NPCs/BP_TurtleWalking.BP_TurtleWalking_C"))))
    (:else)))